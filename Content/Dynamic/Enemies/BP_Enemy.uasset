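; Enemy Blueprint that chases the first player, flashes red when hurt and drops a pickup on death.
; A looping timer re-issues AI MoveTo toward the player pawn, which also restarts on success, while Attack plays a placeholder montage.
; ChangeToHurtMaterial swaps mesh materials and restores them through a short timer.
; CheckDeath tests Health, spawns the drop at the chest socket, destroys the actor and reports the result.
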(event Custom|Chase%20Player
  (AI|AIMoveTo self "0, 0, 0" (Game|Player|GetPlayerPawn 0) 0.0 false
    (:OnSuccess
      (CallFunction|ChasePlayer))))

(event Custom|Attack
  (Animation|Montage|PlayMontage (Variables|Character|GetMesh) "/Game/Static/Characters/Mannequins/Animations/Manny/MM_AttackPlaceholder_Montage.MM_AttackPlaceholder_Montage"))

(event EventBeginPlay
  (Utilities|Time|SetTimerbyEvent (delegate Custom|Chase%20Player) 0.25 true))

(fn ConstructionScript)

(fn ChangetoHurtMaterial
  (bind _mesh (Variables|Character|GetMesh))
  (Rendering|Material|SetMaterial _mesh 0 "/Engine/EngineDebugMaterials/VertexColorViewMode_RedOnly.VertexColorViewMode_RedOnly")
  (Rendering|Material|SetMaterial _mesh 1 "/Engine/EngineDebugMaterials/VertexColorViewMode_RedOnly.VertexColorViewMode_RedOnly")
  (bind _returnvalue (Utilities|Time|SetTimerbyFunctionName 0 "ChangeToBaseMaterial" 0.25))
  (Variables|Default|SetHurtMaterialTimer _returnvalue)
  (return))

(fn ChangetoBaseMaterial
  (bind _mesh (Variables|Character|GetMesh))
  (Rendering|Material|SetMaterial _mesh 0 0)
  (Rendering|Material|SetMaterial _mesh 1 "/Game/Static/Characters/Mannequins/Materials/Instances/Manny/MI_Manny_02.MI_Manny_02")
  (Utilities|Time|ClearandInvalidateTimerbyHandle (Variables|Default|GetHurtMaterialTimer))
  (return))

(fn CheckDeath
  (if (<= (Variables|Default|GetHealth) 0.0)
    (CallFunction|DropPickUp (Variables|Default|GetDrop))
    (Actor|DestroyActor)
    (return true)
    (else
      (return false))))

(fn DropPickUp
  (params (Dropped%20Pick%20Up :type BP%20Pick%20Up%20Class%20Reference))
  (Game|SpawnActorfromClass Dropped%20Pick%20Up (Math|Transform|MakeTransform (Transformation|GetSocketLocation (Variables|Character|GetMesh) "chestSocket")) "Undefined" "MultiplyWithRoot" 0 0)
  (return))